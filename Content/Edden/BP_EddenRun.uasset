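; BP_EddenRun manages an endless-runner style road built from spawned Road tiles, plus a Score.
; BeginPlay calls AddFloor once per NumOfTiles, while Tick prints and increments Score every frame.
; AddFloor holds logic to chain tiles by attach point, and ExtendFloor to add one and cull the oldest.
; Both function bodies are disconnected from their entries, so no tiles spawn or get removed as wired.
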(event EventBeginPlay
  (for _index (range 0 (- (Variables|Default|GetNumOfTiles) 1))
    (CallFunction|AddFloor)))

(event EventTick
  (params (DeltaSeconds :type Float%20%28single-precision%29))
  (bind _score (Variables|Default|GetScore))
  (Development|PrintString (Utilities|String|ToString(Integer) _score))
  (Math|Integer|IncrementInt _score))

(fn ConstructionScript)

(fn AddFloor)

(fn ExtendFloor)