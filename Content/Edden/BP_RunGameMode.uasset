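; Game mode for a two-player local runner that places both run characters at fixed start points, creating the second player at BeginPlay.
; It pre-spawns a chain of Road tiles, each at the previous tile's attach point with Y held fixed.
; ExtendFloor appends a tile, destroys the oldest beyond a set count, and shows the mouse cursor.
; Tick reloads the current level when either pawn drops below a height threshold.
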(event EventBeginPlay
  ;[0 0.03696 0.8385] Sets The Transform For Player 0
  (bind _asbp_run_character (Utilities|Casting|CastToBP_RunCharacter (Game|Player|GetPlayerPawn 0)))
  (Transformation|SetActorTransform _asbp_run_character (Math|Transform|MakeTransform "180.000000,-515.000000,92.000076") false true)
  ;[0 0.7344 0.03188] Creates And Sets The Transform For Player 1
  (bind _returnvalue (Class|GameplayStatics|CreatePlayer -1))
  (Variables|Default|SetplayerTwoRef _returnvalue)
  (bind _asbp_run_character_2 (Utilities|Casting|CastToBP_RunCharacter (Game|Player|GetPlayerPawn 1)))
  (Transformation|SetActorTransform _asbp_run_character_2 (Math|Transform|MakeTransform "115.000000,665.000000,150.000000") false true)
  (for _index (range 0 (+ (Variables|Default|GetNumOfTiles) 9))
    (CallFunction|AddFloor1)))

(event EventTick
  (params (DeltaSeconds :type Float%20%28single-precision%29))
  (for _index (range 0 1)
    (if (<= (.Z (Math|Vector|BreakVector (.Location (Math|Transform|BreakTransform (Transformation|GetActorTransform (Game|Player|GetPlayerPawn _index)))))) 8e+01)
      (bind _returnvalue (Game|GetCurrentLevelName true))
      (Game|OpenLevel(byName) (Utilities|String|StringToName _returnvalue) false))))

(fn ConstructionScript)

(fn AddFloor1
  (bind _returnvalue (Game|SpawnActorfromClass "/Game/Edden/Road.Road_C" (Variables|Default|GetFloorAttachPoint) "Undefined" 0 0))
  (Variables|Default|SetFloorAttachPoint (Math|Transform|MakeTransform (Math|Vector|MakeVector (.X (Math|Vector|BreakVector (.Location (Math|Transform|BreakTransform (Default|GetAttachPoint _returnvalue))))) 5e+02 (.Z (Math|Vector|BreakVector (.Location (Math|Transform|BreakTransform (Default|GetAttachPoint _returnvalue))))))))
  (Utilities|Array|Add (Variables|Default|GetFloorTiles) _returnvalue))

(fn ExtendFloor
  (bind _floortiles (Variables|Default|GetFloorTiles))
  (bind _output (Utilities|Array|Get(acopy) _floortiles))
  (Variables|/Script/Engine.PlayerController|SetbShowMouseCursor (Game|GetPlayerController 0) true)
  (CallFunction|AddFloor1)
  (if (> (Utilities|Array|Length (Variables|Default|GetFloorTiles)) (+ (Variables|Default|GetNumOfTiles) 13))
    (Actor|DestroyActor _output)
    (Utilities|Array|RemoveItem _floortiles _output)))