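; Two-player local runner manager that places two BP_RunCharacter players, creating the second, and builds a separate tiled road for each.
; BeginPlay pre-spawns tiles through AddFloor1, which chains BP_RoadTwo and BP_RoadTwoB from their attach points at fixed lane Y positions.
; ExtendFloor and ExtendFloor1 each extend both roads but trim only their own array's oldest tile past a limit.
; A fall-triggered level restart is present but never runs.
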(event EventBeginPlay
  ;[0 0.03696 0.8385] Sets The Transform For Player 0
  (bind _asbp_run_character (Utilities|Casting|CastToBP_RunCharacter (Game|Player|GetPlayerPawn 0)))
  (Transformation|SetActorTransform _asbp_run_character (Math|Transform|MakeTransform "180.000000,-1000.000000,92.000076") false true)
  ;[0 0.7344 0.03188] Creates And Sets The Transform For Player 1
  (bind _returnvalue (Class|GameplayStatics|CreatePlayer 1))
  (Variables|Default|SetplayerTwoRef _returnvalue)
  (bind _asbp_run_character_2 (Utilities|Casting|CastToBP_RunCharacter (Game|Player|GetPlayerPawn 1)))
  (Transformation|SetActorTransform _asbp_run_character_2 (Math|Transform|MakeTransform "115.000000,665.000000,150.000000") false true)
  (for _index (range 0 (+ (Variables|Default|GetNumOfTiles) 9))
    (CallFunction|AddFloor1)))

(event EventTick
  (params (DeltaSeconds :type Float%20%28single-precision%29)))

(fn ConstructionScript)

(fn AddFloor1
  ;[1 1 1] Side 0
  (bind _returnvalue (Game|SpawnActorfromClass "/Game/Edden/BP_RoadTwo.BP_RoadTwo_C" (Variables|Default|GetFloorAttachPoint) "Undefined" 0 0))
  (Variables|Default|SetFloorAttachPoint (Math|Transform|MakeTransform (Math|Vector|MakeVector (.X (Math|Vector|BreakVector (.Location (Math|Transform|BreakTransform (Default|GetAttachPoint _returnvalue))))) 5e+02 (.Z (Math|Vector|BreakVector (.Location (Math|Transform|BreakTransform (Default|GetAttachPoint _returnvalue))))))))
  (Utilities|Array|Add (Variables|Default|GetFloorTiles) _returnvalue)
  ;[1 1 1] side 1
  (bind _returnvalue_2 (Game|SpawnActorfromClass "/Game/Edden/BP_RoadTwoB.BP_RoadTwoB_C" (Variables|Default|GetFloorAttachPoint1) "Undefined" 0 0))
  (Variables|Default|SetFloorAttachPoint1 (Math|Transform|MakeTransform (Math|Vector|MakeVector (.X (Math|Vector|BreakVector (.Location (Math|Transform|BreakTransform (Default|GetAttachPoint _returnvalue_2))))) -1.5e+03 (.Z (Math|Vector|BreakVector (.Location (Math|Transform|BreakTransform (Default|GetAttachPoint _returnvalue_2))))))))
  (Utilities|Array|Add (Variables|Default|GetFloorTiles1) _returnvalue_2))

(fn ExtendFloor
  (bind _floortiles (Variables|Default|GetFloorTiles))
  (bind _output (Utilities|Array|Get(acopy) _floortiles))
  (Variables|/Script/Engine.PlayerController|SetbShowMouseCursor (Game|GetPlayerController 0) true)
  (CallFunction|AddFloor1)
  (if (> (Utilities|Array|Length (Variables|Default|GetFloorTiles)) (+ (Variables|Default|GetNumOfTiles) 13))
    (Actor|DestroyActor _output)
    (Utilities|Array|RemoveItem _floortiles _output)))

(fn ExtendFloor1
  (bind _floortiles1 (Variables|Default|GetFloorTiles1))
  (bind _output (Utilities|Array|Get(acopy) _floortiles1))
  (Variables|/Script/Engine.PlayerController|SetbShowMouseCursor (Game|GetPlayerController 0) true)
  (CallFunction|AddFloor1)
  (if (> (Utilities|Array|Length (Variables|Default|GetFloorTiles1)) (+ (Variables|Default|GetNumOfTiles) 13))
    (Actor|DestroyActor _output)
    (Utilities|Array|RemoveItem _floortiles1 _output)))