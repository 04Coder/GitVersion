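; Road tile for an endless runner in the BP_TwoPlayer game mode, exposing an attach point transform.
; When a BP_RunCharacter hits the exit box, a macro spawns a random, short-lived object in a random lane ahead of player 0, capped by tagged-actor count.
; The tile then calls ExtendFloor1 on the game mode and destroys the box.
; Construction builds a lane grid of spawn points, but its SpawnObstacles call is disconnected.
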(event OnComponentBeginOverlap(ExitBoxB)
  (params (OverlappedComponent :type Primitive%20Component%20Object%20Reference) (OtherActor :type Actor%20Object%20Reference) (OtherComp :type Primitive%20Component%20Object%20Reference) (OtherBodyIndex :type Integer) (bFromSweep :type Boolean) (SweepResult :type Hit%20Result%20Structure%20%28by%20ref%29))
  (Utilities|Casting|CastToBP_RunCharacter OtherActor)
  (Utilities|SpawnObjectinRoad true 15 0.0 3 0 1e+01
    (:Out
      (bind _asbp_two_player (Utilities|Casting|CastToBP_TwoPlayer (Game|GetGameMode)))
      (Default|ExtendFloor1 _asbp_two_player)
      (Components|DestroyComponent (Variables|Default|GetExitBoxB)))))

(event EventBeginPlay)

(event Collision|EventActorBeginOverlap
  (params (OtherActor :type Actor%20Object%20Reference)))

(fn ConstructionScript
  (CallFunction|InitSpawnPoints))

(fn GetAttachPoint
  (return (Transformation|GetWorldTransform (Variables|Default|GetAttachPoint))))

(fn InitSpawnPoints
  (for _array_element (Variables|Default|GetLanePosition)
    (for _index (range 0 6)
      (bind _returnvalue (AddComponent|AddArrowComponent false (Math|Transform|MakeTransform (Math|Vector|MakeVector (Math|Conversions|ToFloat(Integer) (* _index 200)) _array_element 0.0))))
      (Utilities|Array|Add (Variables|Default|GetSpawnPoints) (Transformation|GetWorldTransform _returnvalue)))))

(fn SpawnObstacles
  (bind _output_get (LocalVariables|SetRandomSpawnPoint (Variables|Default|GetSpawnPoints)))
  (Utilities|Array|Shuffle _output_get)
  (for _index (range 0 (Math|Random|RandomIntegerinRange 0 2))
    (switch int (Math|Random|RandomIntegerinRange 0 4)
      (:0
        (AddComponent|AddChildActorComponent false (Math|Transform|MakeRelativeTransform (Utilities|Array|Get(acopy) (LocalVariables|GetRandomSpawnPoint) _index) (Transformation|GetActorTransform))))
      (:1
        (AddComponent|AddChildActorComponent false (Math|Transform|MakeRelativeTransform (Utilities|Array|Get(acopy) (LocalVariables|GetRandomSpawnPoint) _index) (Transformation|GetActorTransform)))))))